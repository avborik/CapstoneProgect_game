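; DedicatedGameModeBP is a game mode for a dedicated server that tracks connected DedicatedPlayerControllerBP players.
; PostLogin adds each controller to ConnectedPlayers and prints its player ID, and OnLogout removes it.
; A deprecated GetPlayerDetails event fetches player data by GUID through a VaRest GET request, with callbacks that print the inventory and name or a failure.
; GetUserDataFromDB is an empty stub.
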(event Custom|testing
  (Development|PrintString "Testing"))

(event Custom|GetPlayerDetails
  (params (GUID :type String))
  ;[1 -0.4 -0.619] [DEPRECATED] Get Player Information from the Database
  (Variables|Default|SetVaRequest (Class|VaRestRequestJSON|ConstructRequestExt "GET" "x_www_form_urlencoded_url"))
  (EventDispatchers|BindEventtoOnRequestComplete (Variables|Default|GetVaRequest) (delegate Custom|OnRequestComplete))
  (EventDispatchers|BindEventtoOnRequestFail (Variables|Default|GetVaRequest) (delegate Custom|OnRequestFail))
  (bind _returnvalue (Class|VaRestRequestJSON|GetRequestObject (Variables|Default|GetVaRequest)))
  (Class|VaRestJsonObject|SetStringField _returnvalue "getPlayerData" GUID)
  (Class|VaRestRequestJSON|ProcessURL (Variables|Default|GetVaRequest) "schollitt.com/rest/rest.php"))

(event Custom|OnRequestComplete
  (params (Request :type Va%20Rest%20Request%20JSON%20Object%20Reference))
  ;[1 -0.4 -0.619] [DEPRECATED] Get Player Information from the Database
  (bind _returnvalue (Class|VaRestRequestJSON|GetRequestObject Request))
  (for (_array_element _array_index) (Class|VaRestJsonObject|GetObjectArrayField _returnvalue "inventory")
    (Development|PrintString (Utilities|String|Append (Utilities|String|BuildString(Integer) (Class|VaRestJsonObject|GetStringField _array_element "slot") ": " _array_index " ") (Utilities|String|Append "ID: " (Class|VaRestJsonObject|GetStringField _array_element "id")) (Utilities|String|Append ", Quantity: " (Class|VaRestJsonObject|GetStringField _array_element "quantity"))) true true "(R=0.000000,G=0.660000,B=1.000000,A=1.000000)" 3e+01)
    (Development|PrintString (Utilities|String|Append "Joined player name: " (Class|VaRestJsonObject|GetStringField _returnvalue "display")))))

(event Custom|OnRequestFail
  (params (Request :type Va%20Rest%20Request%20JSON%20Object%20Reference))
  ;[1 -0.4 -0.619] [DEPRECATED] Get Player Information from the Database
  (Development|PrintString "Request for player data failed"))

(event EventTick
  (params (DeltaSeconds :type Float%20%28single-precision%29)))

(event EventPostLogin
  (params (NewPlayer :type Player%20Controller%20Object%20Reference))
  (bind _asdedicated_player_controller_bp (Utilities|Casting|CastToDedicatedPlayerControllerBP NewPlayer))
  (Utilities|Array|AddUnique (Variables|Default|GetconnectedPlayers) _asdedicated_player_controller_bp)
  (Development|PrintString (Utilities|String|Append "Added player: " (Utilities|String|ToString(Integer) (Variables|/Script/Engine.PlayerState|GetPlayerId (Variables|/Script/Engine.Controller|GetPlayerState _asdedicated_player_controller_bp))))))

(event EventOnLogout
  (params (ExitingController :type Controller%20Object%20Reference))
  (bind _asdedicated_player_controller_bp (Utilities|Casting|CastToDedicatedPlayerControllerBP ExitingController))
  (Utilities|Array|RemoveItem (Variables|Default|GetconnectedPlayers) _asdedicated_player_controller_bp))

(fn ConstructionScript)

(fn GetUserDatafromDB)