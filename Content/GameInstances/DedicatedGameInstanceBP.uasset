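; Game instance that boots a dedicated server into planeLevel or shows players the login menu, branching on Init.
; GoTo events lazily create and cache menu widgets, while JoinServer shows a loading screen and joins a session.
; CreateNewSession creates one only when the session search fails; dedicated servers destroy theirs on shutdown.
; Network and travel failures route to DisplayErrorMessage, but it and both error-to-string helpers are empty stubs.
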(event Custom|CreateNewSession
  (bind _sessiononlan_ (Variables|SessionSettings|GetSessionOnLan?))
  (bind _maxserverslots (Variables|SessionSettings|GetMaxServerSlots))
  ;[1 1 1] Create a new session if none exist
  (|FindSessions 0 _maxserverslots _sessiononlan_
    (:OnFailure
      (|Session 0 _maxserverslots _sessiononlan_
        (:OnSuccess
          (Game|OpenLevel(byName) "planeLevel" true "PORT=7777"))
        (:OnFailure
          (Development|PrintString "Failed to create session!!" false))))))

(event Custom|JoinServer
  (params (Session :type Blueprint%20Session%20Result%20Structure))
  ;[1 1 1] Attempt to join a session (from parameter)
  (CallFunction|ShowLoadingScreen)
  (|JoinSession (Game|GetPlayerController 0) Session
    (:OnFailure
      (Utilities|DisplayErrorMessage "Failed to join session. Please try again."))))

(event Custom|GoToServerBrowser
  ;[1 1 1] Change the displayed widget to the Server Browser upon request from the Player Controller
  (Utilities|IsValid (Variables|Widgets|GetServerBrowserWB)
    (:Is%20Valid
      _)
    (:Is%20Not%20Valid
      (bind _returnvalue (UserInterface|CreateWidget "/Game/Blueprints/HUD/ServerBrowserWidget.ServerBrowserWidget_C" (Game|GetPlayerController 0)))
      (Variables|Widgets|SetServerBrowserWB _returnvalue)))
  (UserInterface|Viewport|AddtoViewport (Variables|Widgets|GetServerBrowserWB) 0))

(event Custom|ShowLoadingScreen
  ;[1 1 1] Display the loading screen
  (Utilities|IsValid (Variables|Widgets|GetLoadingWB)
    (:Is%20Valid
      _)
    (:Is%20Not%20Valid
      (bind _returnvalue (UserInterface|CreateWidget "/Game/Blueprints/HUD/loadingWidget.loadingWidget_C" (Game|GetPlayerController 0)))
      (Variables|Widgets|SetLoadingWB _returnvalue)))
  (UserInterface|Viewport|AddtoViewport (Variables|Widgets|GetLoadingWB) 0))

(event Custom|initPlayer
  ;[1 1 1] At Init display the main menu to the player
  (CallFunction|GotoLoginMenu))

(event Custom|initServer
  ;[1 1 1] Check for existing sessions, if none create one and open the play level
  (Game|OpenLevel(byName) "planeLevel"))

(event Custom|GoToLoginMenu
  ;[1 1 1] Create the login menu
  (Utilities|IsValid (Variables|Widgets|GetLoginMenuWB)
    (:Is%20Valid
      _)
    (:Is%20Not%20Valid
      (bind _returnvalue (UserInterface|CreateWidget "/Game/Blueprints/HUD/LoginWidget.LoginWidget_C" (Game|GetPlayerController 0)))
      (Variables|Widgets|SetLoginMenuWB _returnvalue)))
  (UserInterface|Viewport|AddtoViewport (Variables|Widgets|GetLoginMenuWB) 0))

(event Custom|HideLoadingScreen
  (bind _loadingwb (Variables|Widgets|GetLoadingWB))
  ;[1 1 1] Remove loadingwidget if it exists
  (Utilities|IsValid _loadingwb
    (:Is%20Valid
      (Widget|RemovefromParent _loadingwb))))

(event Custom|GoToOptionsMenu
  ;[1 1 1] Create the options menu, or display the existing options menu and hide the Main menu
  (Utilities|IsValid (Variables|Widgets|GetOptionsMenuWB)
    (:Is%20Valid
      _)
    (:Is%20Not%20Valid
      (bind _returnvalue (UserInterface|CreateWidget "/Game/Blueprints/HUD/OptionsMenuWidget.OptionsMenuWidget_C" (Game|GetPlayerController 0)))
      (Variables|Widgets|SetOptionsMenuWB _returnvalue)))
  (UserInterface|Viewport|AddtoViewport (Variables|Widgets|GetOptionsMenuWB) 0))

(event Custom|GoToMainMenu
  ;[1 1 1] Create the MainMenu widget and display on clients
  (Utilities|IsValid (Variables|Widgets|GetMainMenuWB)
    (:Is%20Valid
      _)
    (:Is%20Not%20Valid
      (bind _returnvalue (UserInterface|CreateWidget "/Game/Blueprints/HUD/MainMenuWidget.MainMenuWidget_C" (Game|GetPlayerController 0)))
      (Variables|Widgets|SetMainMenuWB _returnvalue)))
  (UserInterface|Viewport|AddtoViewport (Variables|Widgets|GetMainMenuWB) 0))

(event EventInit
  ;[1 1 1] Run the initialise functions for server or client
  (if (Networking|IsDedicatedServer)
    (CallFunction|InitServer)
    (else
      (CallFunction|InitPlayer))))

(event EventHandleTravelError
  (params (FailureType :type ETravelFailure%20Enum :default "NoLevel"))
  ;[1 1 1] Handle travel errors and display to client
  (Utilities|DisplayErrorMessage (CallFunction|TravelErrortoString FailureType)))

(event EventShutdown
  ;[1 1 1] Destroy session on shutdown
  (if (Networking|IsDedicatedServer)
    (|DestroySession (Game|GetPlayerController 0))))

(event EventHandleNetworkError
  (params (FailureType :type ENetworkFailure%20Enum :default "NetDriverAlreadyExists") (bIsServer :type Boolean))
  ;[1 1 1] Handle network errors and display to client
  (if (not bIsServer)
    (Utilities|DisplayErrorMessage (CallFunction|NetworkErrortoString FailureType))))

(fn NetworkErrortoString
  (params (ErrorType :type ENetworkFailure%20Enum :default "NetDriverAlreadyExists")))

(fn TravelErrortoString
  (params (Error%20type :type ETravelFailure%20Enum :default "NoLevel")))