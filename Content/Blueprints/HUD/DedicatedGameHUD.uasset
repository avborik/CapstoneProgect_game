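; DedicatedGameHUD is a HUD Blueprint that owns the player's on-screen widgets: main HUD, coordinates, ping, hotbar and tutorial.
; Init creates each widget for the owning player controller, adds it to the viewport, offsets the tutorial's position and returns all references to the caller.
; A SetVisibility event shows or hides all five stored widgets together.
; BeginPlay is empty, so the file itself never calls Init.
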(event Custom|SetVisibility
  (params (Visible :type Boolean))
  (bind _coordinateswidget (Variables|Default|GetCoordinatesWidget))
  (bind _pingwidget (Variables|Default|GetPingWidget))
  (bind _hotbarwidget (Variables|Default|GetHotbarWidget))
  (bind _mainhud (Variables|Default|GetMainHUD))
  (bind _tutorialwidget (Variables|Default|GetTutorialWidget))
  (if Visible
    (Widget|SetVisibility _mainhud "Visible")
    (Widget|SetVisibility _pingwidget "Visible")
    (Widget|SetVisibility _coordinateswidget "Visible")
    (Widget|SetVisibility _hotbarwidget "Visible")
    (Widget|SetVisibility _tutorialwidget "Visible")
    (else
      (Widget|SetVisibility _mainhud "Hidden")
      (Widget|SetVisibility _pingwidget "Hidden")
      (Widget|SetVisibility _coordinateswidget "Hidden")
      (Widget|SetVisibility _hotbarwidget "Hidden")
      (Widget|SetVisibility _tutorialwidget "Hidden"))))

(event EventBeginPlay)

(fn ConstructionScript)

(fn Init
  (bind _returnvalue (Game|Player|GetOwningPlayerController))
  (bind _returnvalue_2 (UserInterface|CreateWidget "/Game/Blueprints/HUD/MainUI/MainHUD.MainHUD_C" _returnvalue))
  (bind _output_get (Variables|Default|SetMainHUD _returnvalue_2))
  (UserInterface|Viewport|AddtoViewport _output_get 0)
  (bind _returnvalue_3 (UserInterface|CreateWidget "/Game/Blueprints/HUD/CoordsWidget.CoordsWidget_C" _returnvalue))
  (bind _output_get_2 (Variables|Default|SetCoordinatesWidget _returnvalue_3))
  (UserInterface|Viewport|AddtoViewport _output_get_2 0)
  (bind _returnvalue_4 (UserInterface|CreateWidget "/Game/Blueprints/HUD/PingWidget.PingWidget_C" _returnvalue))
  (bind _output_get_3 (Variables|Default|SetPingWidget _returnvalue_4))
  (UserInterface|Viewport|AddtoViewport _output_get_3 0)
  (bind _returnvalue_5 (UserInterface|CreateWidget "/Game/Blueprints/HUD/HotbarWidget.HotbarWidget_C" _returnvalue))
  (bind _output_get_4 (Variables|Default|SetHotbarWidget _returnvalue_5))
  (UserInterface|Viewport|AddtoViewport _output_get_4 0)
  (bind _returnvalue_6 (UserInterface|CreateWidget "/Game/Blueprints/HUD/Tutorial/W_tutorial.W_tutorial_C" _returnvalue))
  (bind _output_get_5 (Variables|Default|SetTutorialWidget _returnvalue_6))
  (UserInterface|Viewport|AddtoViewport _output_get_5 0)
  (Default|SetPosition _output_get_5 0.0 2e+02)
  (return _output_get _output_get_2 _output_get_3 _output_get_4 _returnvalue_6))