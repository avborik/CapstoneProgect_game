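; Slot-based inventory that stores item classes and stack counts, reading name, weight and stack limit from each class's defaults.
; Init fills the array with empty slots, and PrintInventory prints each slot for debugging.
; AddItemToInventory first checks current weight against MaxWeight, then increments a matching partial stack or takes the first empty slot.
; Macros handle the weight and stack checks, while IsStackable and SwitchHasAuthority are defined but unused here.
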(event Custom|Init
  (params (slotCount :type Integer))
  (bind _slots (Variables|Default|GetSlots))
  (bind _returnvalue (Utilities|Array|Length _slots))
  (Utilities|Array|Clear _slots)
  (if (< _returnvalue slotCount) :!label _label
    (Utilities|Array|Add (Variables|Default|GetSlots) (Utilities|Struct|MakeInventorySlot "/Game/Blueprints/Stock_Objects/BaseObject/baseObject.baseObject_C"))
    (goto _label)
    (else
      (Development|PrintString 0 (Utilities|String|BuildString(Integer) "Inventory init complete, added " "" _returnvalue " empty slots.")))))

(event Custom|PrintInventory
  (for (_array_element _array_index) (Variables|Default|GetSlots)
    (Development|PrintString 0 (Utilities|String|Append (Utilities|String|BuildString(Integer) "" "Item " _array_index ": ") (.ObjectName (Utilities|GetClassDefaults (.Item (Utilities|Struct|BreakInventorySlot _array_element)))) " (count: " (Utilities|String|ToString(Integer) (.StackCount (Utilities|Struct|BreakInventorySlot _array_element))) ")") true true "(R=0.106177,G=1.000000,B=0.000000,A=1.000000)" 3e+01)))

(fn AddItemtoInventory
  (params (ItemToAdd :type Base%20Object%20Class%20Reference))
  (bind _slots (Variables|Default|GetSlots))
  (Utilities|IsUnderWeightLimit
    (:Out
      (bind _index (Utilities|HasPartialStack ItemToAdd)
        (:True
          (Math|Integer|IncrementInt (.StackCount (Utilities|Struct|BreakInventorySlot (Utilities|Array|Get(acopy) _slots _index)))
            (:%20%20
              (LocalVariables|SetItem%20Added true :!label _label))))
        (:False
          (bind (_hasfoundemptyslot1 _array_index) (CallFunction|GetEmptyStack))
          (if _hasfoundemptyslot1
            (Utilities|Array|SetArrayElem _slots _array_index (Utilities|Struct|MakeInventorySlot ItemToAdd _index))
            (goto _label)
            (else
              (LocalVariables|SetItem%20Added false)))))
      (return (LocalVariables|GetItem%20Added)))))

(fn GetEmptyStack
  (bind (_array_element _array_index) (Utilities|Array|ForEachLoopwithBreak (Variables|Default|GetSlots) :!label _label)
    (:LoopBody
      (bind _output_get (LocalVariables|SetHasFoundEmptySlot (== (.StackCount (Utilities|Struct|BreakInventorySlot _array_element)) 0)))
      (if _output_get
        (goto _label Break)))
    (:Completed
      (return (LocalVariables|GetHasFoundEmptySlot) _array_index))))