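; Base inventory Blueprint that stores items as a fixed number of slots, each holding an item class and stack count.
; Init fills the slots with empty placeholders, and item limits and weights come from class defaults.
; Adding runs only on authority, gated by a weight check, then tries a partial stack before an empty slot.
; Functions also set slots, decrement stacks back to empty, and print contents for debugging.
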(event Custom|Init
  (bind _invslots (Variables|Editable|GetInvSlots))
  (bind _returnvalue (Utilities|Array|Length _invslots))
  (Utilities|Array|Clear _invslots)
  (if (< _returnvalue (Variables|Editable|GetSlotCount)) :!label _label
    (Utilities|Array|Add (Variables|Editable|GetInvSlots) (Utilities|Struct|MakeInventoryStruct "/Game/Blueprints/Stock_Objects/BaseObject/emptyObject.emptyObject_C"))
    (goto _label)
    (else
      (Development|PrintString (Utilities|String|BuildString(Integer) "Inventory init complete, added " "" _returnvalue " empty slots.")))))

(event Custom|PrintInventory
  (for (_array_element _array_index) (Variables|Editable|GetInvSlots)
    (Development|PrintString (Utilities|String|Append (Utilities|String|BuildString(Integer) "" "Item " _array_index ": ") "" " (count: " (Utilities|String|ToString(Integer) (.StackCount (Utilities|Struct|BreakInventoryStruct _array_element))) ") " (Utilities|GetDisplayName (Utilities|Struct|BreakImageContainer (.ImageContainer (Utilities|GetClassDefaults (.ItemType (Utilities|Struct|BreakInventoryStruct _array_element))))))) true true "(R=0.106177,G=1.000000,B=0.000000,A=1.000000)" 3e+01)))

(fn ConstructionScript)

(fn AddItemtoInventory
  (params (In%20Actor :type Base%20Object%20CPP%20Class%20Reference))
  (bind _invslots (Variables|Editable|GetInvSlots))
  (Networking|SwitchHasAuthority
    (:Authority
      (Utilities|IsUnderWeightLimit
        (:true
          (bind _index (Utilities|HasPartialStack In%20Actor)
            (:True
              (Math|Integer|IncrementInt (.StackCount (Utilities|Struct|BreakInventoryStruct (Utilities|Array|Get(acopy) _invslots _index)))
                (:%20%20
                  (LocalVariables|SetIndexAdded _index)
                  (LocalVariables|SetitemAdded true :!label _label))))
            (:false
              (bind (_hasfoundemptyslot1 _array_index) (CallFunction|GetEmptyStack))
              (if _hasfoundemptyslot1
                (Utilities|Array|SetArrayElem _invslots _array_index (Utilities|Struct|MakeInventoryStruct In%20Actor _index))
                (LocalVariables|SetIndexAdded _array_index)
                (goto _label)
                (else
                  (LocalVariables|SetitemAdded false)))))
          (return (LocalVariables|GetitemAdded) (LocalVariables|GetIndexAdded)))))))

(fn GetEmptyStack
  (bind (_array_element _array_index) (Utilities|Array|ForEachLoopwithBreak 0 :!label _label)
    (:LoopBody
      (bind _output_get (LocalVariables|SetHasFoundEmptySlot (== (.StackCount (Utilities|Struct|BreakInventoryStruct _array_element)) 0)))
      (if _output_get
        (goto _label Break)))
    (:Completed
      (return (LocalVariables|GetHasFoundEmptySlot) _array_index))))

(fn SetItemSlot
  (params (Item :type Base%20Object%20CPP%20Class%20Reference) (Slot :type Integer) (Quantity :type Integer) (Force :type Boolean))
  (bind _maxstacksize (Utilities|GetClassDefaults Item))
  (bind _invslots (Variables|Editable|GetInvSlots))
  (bind _output (Utilities|Array|Get(acopy) _invslots Slot))
  (bind (_itemtype _stackcount) (Utilities|Struct|BreakInventoryStruct _output))
  (LocalVariables|SetfinalQuantity Quantity)
  (if Force
    (|SetBy-RefVar _itemtype Item :!label _label)
    (|SetBy-RefVar _stackcount (LocalVariables|GetfinalQuantity))
    (return _output Slot)
    (elif (<= Slot (Utilities|Array|Length (Variables|Editable|GetInvSlots)))
      (if (>= _maxstacksize (LocalVariables|GetfinalQuantity))
        (goto _label)
        (else
          (LocalVariables|SetfinalQuantity _maxstacksize)
          (goto _label))))))

(fn RemoveItem
  (params (Slot%20Index :type Integer))
  (bind _invslots (Variables|Editable|GetInvSlots))
  (bind _invslots_2 (Variables|Editable|GetInvSlots))
  (bind _output (Utilities|Array|Get(acopy) _invslots_2 Slot%20Index))
  (bind _output_2 (Utilities|Array|Get(acopy) _invslots Slot%20Index))
  (bind (_itemtype _stackcount) (Utilities|Struct|BreakInventoryStruct _output))
  (bind (_itemtype_2 _stackcount_2) (Utilities|Struct|BreakInventoryStruct _output_2))
  (if (> _stackcount 0)
    (bind _result (Math|Integer|DecrementInt _stackcount)
      (:%20%20
        (if (== _result 0)
          (|SetBy-RefVar _itemtype "/Game/Blueprints/Stock_Objects/BaseObject/emptyObject.emptyObject_C")
          (Development|PrintString (Utilities|String|Append (Utilities|String|ToString(Integer) (.ObjectID (Utilities|GetClassDefaults _itemtype_2))) "," (Utilities|String|ToString(Integer) _stackcount_2) ",,"))
          (return _output_2))))))