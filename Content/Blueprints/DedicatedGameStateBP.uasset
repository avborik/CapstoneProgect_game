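; DedicatedGameStateBP is a game state that keeps a shared time-of-day counter and holds a table of four player shops.
; Tick advances the counter once per frame, not by elapsed time, wrapping at 86400 and calling CallNewDay at 50400.
; CallNewDay walks PlayerArray, reaching each player state's owning controller to run its new-day logic.
; Other events fill the shop table and override the time, which a getter exposes.
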(event Custom|CallNewDay
  (for _array_element (Variables|Default|GetPlayerArray)
    (bind _asdedicated_player_state_bp (Utilities|Casting|CastToDedicatedPlayerStateBP _array_element))
    (bind _asdedicated_player_controller_bp (Utilities|Casting|CastToDedicatedPlayerControllerBP (Components|GetOwner _asdedicated_player_state_bp)))
    (Development|PrintString (Variables|/Game/Blueprints/Character/DedicatedPlayerControllerBP.DedicatedPlayerControllerBP_C|GetGUIDString _asdedicated_player_controller_bp))
    (Default|RunNewDay _asdedicated_player_controller_bp)))

(event Custom|SetCurrentTime
  (params (NewTime :type Integer))
  (Variables|Default|SetcurrentTime NewTime)
  (Development|PrintString "bitch"))

(event Custom|InitPlayerShopList
  (params (Shop1 :type Shop%20Actor%20Object%20Reference) (Shop2 :type Shop%20Actor%20Object%20Reference) (Shop3 :type Shop%20Actor%20Object%20Reference) (Shop4 :type Shop%20Actor%20Object%20Reference))
  (bind _playershoptable (Variables|Default|GetPlayerShopTable))
  (|SetBy-RefVar (.Shop (Utilities|Struct|BreakPlayerStore (Utilities|Array|Get(acopy) _playershoptable))) Shop1)
  (|SetBy-RefVar (.Shop (Utilities|Struct|BreakPlayerStore (Utilities|Array|Get(acopy) _playershoptable 1))) Shop2)
  (|SetBy-RefVar (.Shop (Utilities|Struct|BreakPlayerStore (Utilities|Array|Get(acopy) _playershoptable 2))) Shop3)
  (|SetBy-RefVar (.Shop (Utilities|Struct|BreakPlayerStore (Utilities|Array|Get(acopy) _playershoptable 3))) Shop4))

(event EventTick
  (params (DeltaSeconds :type Float%20%28single-precision%29))
  (if (< (Variables|Default|GetcurrentTime) 86400)
    (bind _result (Math|Integer|IncrementInt (Variables|Default|GetcurrentTime))
      (:%20%20
        (if (== _result 50400)
          (CallFunction|CallNewDay))))
    (else
      (Variables|Default|SetcurrentTime 0))))

(fn ConstructionScript)

(fn GetCurrentTime
  (return (Variables|Default|GetcurrentTime)))