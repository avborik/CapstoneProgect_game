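; Dedicated-server game state that runs the shared day clock, player shop assignments and AI bot spawning.
; Each tick advances a counter that wraps at 86400 and triggers RunNewDay on every player controller at 50400.
; A six-slot shop table backs spawn requests, GUID player lookup and authority-only security/banner upgrades, alongside an experience-to-level lookup.
; Capped AI spawning picks random spawn points, speeds and directions, but its tick call is unwired.
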(event Custom|initAISpawnPoints
  (params (Point1 :type AI%20Stops%20Object%20Reference) (Point2 :type AI%20Stops%20Object%20Reference) (Point3 :type AI%20Stops%20Object%20Reference) (Point4 :type AI%20Stops%20Object%20Reference) (Point5 :type AI%20Stops%20Object%20Reference) (Point6 :type AI%20Stops%20Object%20Reference))
  (bind _aispawnlocations (Variables|Default|GetAISpawnLocations))
  (Utilities|Array|SetArrayElem _aispawnlocations 0 Point1)
  (Utilities|Array|SetArrayElem _aispawnlocations 1 Point2)
  (Utilities|Array|SetArrayElem _aispawnlocations 2 Point3)
  (Utilities|Array|SetArrayElem _aispawnlocations 3 Point4)
  (Utilities|Array|SetArrayElem _aispawnlocations 4 Point5)
  (Utilities|Array|SetArrayElem _aispawnlocations 5 Point6))

(event Custom|RandomlySpawnAI
  (bind _returnvalue (Game|SpawnActorfromClass "/Game/Blueprints/World_Objects/AI/AIBot2.AIBot2_C" (Math|Transform|MakeTransform "-338.000000,-7851.000000,2000.000000") "AdjustIfPossibleButAlwaysSpawn" 0 (Utilities|Array|Get(acopy) (Variables|Default|GetAISpawnLocations) (Math|Random|RandomInteger 5)) (Math|Random|RandomFloatinRange 1.5e+02 3.5e+02) (Math|Random|RandomBool) 0))
  (Utilities|Array|Add (Variables|Default|GetActiveAI) _returnvalue))

(event Custom|CallNewDay
  (for _array_element (Variables|Default|GetPlayerArray)
    (bind _asdedicated_player_state_bp (Utilities|Casting|CastToDedicatedPlayerStateBP _array_element))
    (bind _asdedicated_player_controller_bp (Utilities|Casting|CastToDedicatedPlayerControllerBP (Components|GetOwner _asdedicated_player_state_bp)))
    (Development|PrintString (Variables|/Game/Blueprints/Character/DedicatedPlayerControllerBP.DedicatedPlayerControllerBP_C|GetGUIDString _asdedicated_player_controller_bp))
    (Default|RunNewDay _asdedicated_player_controller_bp)))

(event Custom|SetCurrentTime
  (params (NewTime :type Integer))
  (Variables|Default|SetcurrentTime NewTime)
  (Development|PrintString "bitch"))

(event Custom|InitPlayerShopList
  (params (Shop1 :type Shop%20Actor%20Object%20Reference) (Shop2 :type Shop%20Actor%20Object%20Reference) (Shop3 :type Shop%20Actor%20Object%20Reference) (Shop4 :type Shop%20Actor%20Object%20Reference) (Shop5 :type Shop%20Actor%20Object%20Reference) (Shop6 :type Shop%20Actor%20Object%20Reference))
  (bind _playershoptable (Variables|Default|GetPlayerShopTable))
  (|SetBy-RefVar (.Shop (Utilities|Struct|BreakPlayerStore (Utilities|Array|Get(acopy) _playershoptable))) Shop1)
  (|SetBy-RefVar (.Shop (Utilities|Struct|BreakPlayerStore (Utilities|Array|Get(acopy) _playershoptable 1))) Shop2)
  (|SetBy-RefVar (.Shop (Utilities|Struct|BreakPlayerStore (Utilities|Array|Get(acopy) _playershoptable 2))) Shop3)
  (|SetBy-RefVar (.Shop (Utilities|Struct|BreakPlayerStore (Utilities|Array|Get(acopy) _playershoptable 3))) Shop4)
  (|SetBy-RefVar (.Shop (Utilities|Struct|BreakPlayerStore (Utilities|Array|Get(acopy) _playershoptable 4))) Shop5)
  (|SetBy-RefVar (.Shop (Utilities|Struct|BreakPlayerStore (Utilities|Array|Get(acopy) _playershoptable 5))) Shop6))

(event Custom|TickTime
  (if (< (Variables|Default|GetcurrentTime) 86400)
    (bind _result (Math|Integer|IncrementInt (Variables|Default|GetcurrentTime))
      (:%20%20
        (if (== _result 50400)
          (CallFunction|CallNewDay))))
    (else
      (Variables|Default|SetcurrentTime 0))))

(event Custom|tickSpawn
  (bind _result (Math|Integer|IncrementInt (Variables|Default|GetEmptyTickCount))
    (:%20%20
      (if (== _result 10)
        (Variables|Default|SetEmptyTickCount 0)
        (if (< (Utilities|Array|Length (Variables|Default|GetActiveAI)) (Variables|Default|GetMaxActiveAI))
          (CallFunction|RandomlySpawnAI)
          (Development|PrintString "SpawnNewAI"))
        (else
          (Development|PrintString "tickNoSpawn"))))))

(event EventTick
  (params (DeltaSeconds :type Float%20%28single-precision%29))
  (CallFunction|TickTime))

(fn ConstructionScript)

(fn GetCurrentTime
  (return (Variables|Default|GetcurrentTime)))

(fn RequestSpawn
  (params (ShopIndex :type Integer) (RequestingPlayer :type Dedicated%20Player%20Controller%20BP%20Object%20Reference))
  (bind _returnvalue (- ShopIndex 1))
  (bind _playershoptable (Variables|Default|GetPlayerShopTable))
  (bind _output (Utilities|Array|Get(acopy) _playershoptable _returnvalue))
  (bind (_player _shop) (Utilities|Struct|BreakPlayerStore _output))
  (Utilities|IsValid _player
    (:Is%20Valid
      (return false (Math|Transform|MakeTransform "0, 0,130.000000")))
    (:Is%20Not%20Valid
      (|SetBy-RefVar _player RequestingPlayer)
      (Variables|/Game/Blueprints/World_Objects/ShopActor.ShopActor_C|SetOwningPlayerGUID _shop (Variables|/Game/Blueprints/Character/DedicatedPlayerControllerBP.DedicatedPlayerControllerBP_C|GetGUIDString RequestingPlayer))
      (return true (Transformation|GetWorldTransform (Variables|/Game/Blueprints/World_Objects/ShopActor.ShopActor_C|GetSpawnPoint _shop))))))

(fn GetPlayer
  (params (GUID :type String))
  (Networking|SwitchHasAuthority
    (:Authority
      (bind _array_element (Utilities|Array|ForEachLoopwithBreak (Variables|Default|GetPlayerShopTable) :!label _label)
        (:LoopBody
          (if (Utilities|Enum|Equal(Enum) (Variables|/Game/Blueprints/Character/DedicatedPlayerControllerBP.DedicatedPlayerControllerBP_C|GetGUIDString (.Player (Utilities|Struct|BreakPlayerStore _array_element))) GUID)
            (Utilities|FlowControl|Sequence
              (:then_0
                (goto _label Break))
              (:then_1
                (return (.Player (Utilities|Struct|BreakPlayerStore _array_element)))))))))))

(fn UpdateSecurityLevel
  (params (player :type Dedicated%20Player%20Controller%20BP%20Object%20Reference) (New%20Level :type Integer))
  (Networking|SwitchHasAuthority
    (:Authority
      (bind _array_element (Utilities|Array|ForEachLoopwithBreak (Variables|Default|GetPlayerShopTable) :!label _label)
        (:LoopBody
          (if (== (.Player (Utilities|Struct|BreakPlayerStore _array_element)) player)
            (Utilities|FlowControl|Sequence
              (:then_0
                (goto _label Break))
              (:then_1
                (Default|SetSecurity (.Shop (Utilities|Struct|BreakPlayerStore _array_element)) New%20Level)))))))))

(fn UpdateBannerLevel
  (params (Player :type Dedicated%20Player%20Controller%20BP%20Object%20Reference) (New%20Level :type Integer))
  (Networking|SwitchHasAuthority
    (:Authority
      (bind _array_element (Utilities|Array|ForEachLoopwithBreak (Variables|Default|GetPlayerShopTable) :!label _label)
        (:LoopBody
          (if (== (.Player (Utilities|Struct|BreakPlayerStore _array_element)) Player)
            (Utilities|FlowControl|Sequence
              (:then_0
                (goto _label Break))
              (:then_1
                (Default|SetBanner (.Shop (Utilities|Struct|BreakPlayerStore _array_element)) New%20Level)))))))))

(fn GetLevelfromExp
  (params (Experience :type Integer))
  (bind (_array_element _array_index) (Utilities|Array|ForEachLoopwithBreak (Variables|Default|GetLevelLookupTable) :!label _label)
    (:LoopBody
      (if (>= Experience (.Experience (Utilities|Struct|BreakExpLevel _array_element)))
        (LocalVariables|SetCurrentLevel (.Level (Utilities|Struct|BreakExpLevel _array_element)))
        (else
          (Utilities|FlowControl|Sequence
            (:then_0
              (goto _label Break))
            (:then_1
              (bind _output_get (LocalVariables|SetRemainder (- Experience (.Experience (Utilities|Struct|BreakExpLevel (Utilities|Array|Get(acopy) (Variables|Default|GetLevelLookupTable) (- _array_index 1)))))))
              (return (LocalVariables|GetCurrentLevel) (/ (Math|Conversions|ToFloat(Integer) _output_get) (Math|Conversions|ToFloat(Integer) (- (.Experience (Utilities|Struct|BreakExpLevel _array_element)) (.Experience (Utilities|Struct|BreakExpLevel (Utilities|Array|Get(acopy) (Variables|Default|GetLevelLookupTable) (- _array_index 1)))))))))))))))