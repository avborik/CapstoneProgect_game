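; Trigger actor for a shop's double sliding doors that open when an actor overlaps it while the shop is open.
; BeginPlay caches each door's starting relative location, and two timelines add their offset tracks to those positions to slide the doors.
; On end overlap, the timelines reverse only once the collision component has no remaining overlapping actors and the shop is still open.
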(event EventBeginPlay
  (if (Math|Vector|Equal(Vector) (Variables|Default|GetleftDoorStartLocation) "0, 0, 0" 0.0001)
    (Variables|Default|SetleftDoorStartLocation (Variables|/Script/Engine.SceneComponent|GetRelativeLocation (Variables|Default|GetDoorLeft)))
    (Variables|Default|SetrightDoorStartLocation (Variables|/Script/Engine.SceneComponent|GetRelativeLocation (Variables|Default|GetDoorRight)))))

(event Collision|EventActorBeginOverlap
  (params (OtherActor :type Actor%20Object%20Reference))
  (if (Variables|Default|GetIsShopOpen)
    (Utilities|FlowControl|Sequence
      (:then_0
        (bind _newtrack_0 (Timeline|LeftDoorOpen Play)
          (:Update
            (Transformation|SetRelativeLocation (Variables|Default|GetDoorLeft) (+ _newtrack_0 (Variables|Default|GetleftDoorStartLocation)) false false))))
      (:then_1
        (bind _newtrack_0_2 (Timeline|RightDoorOpen Play)
          (:Update
            (Transformation|SetRelativeLocation (Variables|Default|GetDoorRight) (+ _newtrack_0_2 (Variables|Default|GetrightDoorStartLocation)) false false)))))))

(event Collision|EventActorEndOverlap
  (params (OtherActor :type Actor%20Object%20Reference))
  (if (Variables|Default|GetIsShopOpen)
    (if (== (Utilities|Array|Length (Collision|GetOverlappingActors (Variables|Default|GetCollisionComponent) 0 :!class /Script/Engine.PrimitiveComponent)) 0)
      (Utilities|FlowControl|Sequence
        (:then_0
          (bind _newtrack_0 (Timeline|LeftDoorOpen Reverse)
            (:Update
              (Transformation|SetRelativeLocation (Variables|Default|GetDoorLeft) (+ _newtrack_0 (Variables|Default|GetleftDoorStartLocation)) false false))))
        (:then_1
          (bind _newtrack_0_2 (Timeline|RightDoorOpen Reverse)
            (:Update
              (Transformation|SetRelativeLocation (Variables|Default|GetDoorRight) (+ _newtrack_0_2 (Variables|Default|GetrightDoorStartLocation)) false false))))))))

(event EventTick
  (params (DeltaSeconds :type Float%20%28single-precision%29)))

(fn ConstructionScript)