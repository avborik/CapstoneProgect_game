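; IslandShelves is a world-object shelf unit that populates itself with six ShelfSlot actors.
; On BeginPlay, Init spawns one slot at each SlotLocation component's world transform, owned by the shelf and stored in its own SlotItem variable.
; Each slot is set to replicate, though spawning has no authority check.
; The construction script is empty, and the nodes that would fill the Slots array are disconnected.
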(event Custom|Init
  (bind _returnvalue (Game|SpawnActorfromClass "/Game/Blueprints/World_Objects/ShelfSlot.ShelfSlot_C" (Transformation|GetWorldTransform (Variables|Default|GetSlotLocation0)) "AlwaysSpawn" self 0))
  (Networking|SetReplicates _returnvalue true)
  (Variables|SlotItems|SetSlotItem0 _returnvalue)
  (bind _returnvalue_2 (Game|SpawnActorfromClass "/Game/Blueprints/World_Objects/ShelfSlot.ShelfSlot_C" (Transformation|GetWorldTransform (Variables|Default|GetSlotLocation1)) "AlwaysSpawn" self 0))
  (Networking|SetReplicates _returnvalue_2 true)
  (Variables|SlotItems|SetSlotItem1 _returnvalue_2)
  (bind _returnvalue_3 (Game|SpawnActorfromClass "/Game/Blueprints/World_Objects/ShelfSlot.ShelfSlot_C" (Transformation|GetWorldTransform (Variables|Default|GetSlotLocation2)) "AlwaysSpawn" self 0))
  (Networking|SetReplicates _returnvalue_3 true)
  (Variables|SlotItems|SetSlotItem2 _returnvalue_3)
  (bind _returnvalue_4 (Game|SpawnActorfromClass "/Game/Blueprints/World_Objects/ShelfSlot.ShelfSlot_C" (Transformation|GetWorldTransform (Variables|Default|GetSlotLocation3)) "AlwaysSpawn" self 0))
  (Networking|SetReplicates _returnvalue_4 true)
  (Variables|SlotItems|SetSlotItem3 _returnvalue_4)
  (bind _returnvalue_5 (Game|SpawnActorfromClass "/Game/Blueprints/World_Objects/ShelfSlot.ShelfSlot_C" (Transformation|GetWorldTransform (Variables|Default|GetSlotLocation4)) "AlwaysSpawn" self 0))
  (Networking|SetReplicates _returnvalue_5 true)
  (Variables|SlotItems|SetSlotItem4 _returnvalue_5)
  (bind _returnvalue_6 (Game|SpawnActorfromClass "/Game/Blueprints/World_Objects/ShelfSlot.ShelfSlot_C" (Transformation|GetWorldTransform (Variables|Default|GetSlotLocation5)) "AlwaysSpawn" self 0))
  (Networking|SetReplicates _returnvalue_6 true)
  (Variables|SlotItems|SetSlotItem5 _returnvalue_6))

(event EventBeginPlay
  (CallFunction|Init))

(fn ConstructionScript)