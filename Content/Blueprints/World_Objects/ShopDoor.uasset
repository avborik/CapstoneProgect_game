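; Interactable double door that lets the owning player open or close a shop.
; Interaction routes through the player's ToggleShopDoors, and the toggle event checks the player's GUID against the owning ShopActor before switching both the door and shop state.
; Two timelines slide the door halves relative to start locations cached on BeginPlay, playing to open and reversing to close while the popup prompt updates.
; A tick-counted cooldown, frame-rate dependent, blocks rapid toggling.
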(event Custom|OpenShop
  (CallFunction|SetPopupMessage "Press E to Close Shop")
  (Utilities|FlowControl|Sequence
    (:then_0
      (bind _newtrack_0 (Timeline|LeftDoorOpen Play)
        (:Update
          (Transformation|SetRelativeLocation (Variables|Default|GetDoorLeft) (+ _newtrack_0 (Variables|Default|GetleftDoorStartLocation)) false false))))
    (:then_1
      (bind _newtrack_0_2 (Timeline|RightDoorOpen Play)
        (:Update
          (Transformation|SetRelativeLocation (Variables|Default|GetDoorRight) (+ _newtrack_0_2 (Variables|Default|GetrightDoorStartLocation)) false false))))))

(event Custom|CloseShop
  (CallFunction|SetPopupMessage "Press E to Open Shop")
  (Utilities|FlowControl|Sequence
    (:then_0
      (bind _newtrack_0 (Timeline|LeftDoorOpen Reverse)
        (:Update
          (Transformation|SetRelativeLocation (Variables|Default|GetDoorLeft) (+ _newtrack_0 (Variables|Default|GetleftDoorStartLocation)) false false))))
    (:then_1
      (bind _newtrack_0_2 (Timeline|RightDoorOpen Reverse)
        (:Update
          (Transformation|SetRelativeLocation (Variables|Default|GetDoorRight) (+ _newtrack_0_2 (Variables|Default|GetrightDoorStartLocation)) false false))))))

(event Custom|ToggleShopOpenClose
  (params (RequestingPlayer :type Dedicated%20Player%20Controller%20BP%20Object%20Reference))
  (if (== (Variables|Default|GetDoorToggleCooldown) 0)
    (bind _asshop_actor (Utilities|Casting|CastToShopActor (Components|GetOwner)))
    (if (Utilities|Enum|Equal(Enum) (Variables|/Game/Blueprints/Character/DedicatedPlayerControllerBP.DedicatedPlayerControllerBP_C|GetGUIDString RequestingPlayer) (Variables|/Game/Blueprints/World_Objects/ShopActor.ShopActor_C|GetOwningPlayerGUID _asshop_actor))
      (if (Variables|/Game/Blueprints/World_Objects/ShopActor.ShopActor_C|GetIsShopOpen _asshop_actor)
        (CallFunction|CloseShop)
        (Default|CloseShop _asshop_actor)
        (else
          (CallFunction|OpenShop)
          (Default|OpenShop _asshop_actor)))
      (Variables|Default|SetDoorToggleCooldown 60))))

(event EventBeginPlay
  (if (Math|Vector|Equal(Vector) (Variables|Default|GetleftDoorStartLocation) "0, 0, 0" 0.0001)
    (Variables|Default|SetleftDoorStartLocation (Variables|/Script/Engine.SceneComponent|GetRelativeLocation (Variables|Default|GetDoorLeft)))
    (Variables|Default|SetrightDoorStartLocation (Variables|/Script/Engine.SceneComponent|GetRelativeLocation (Variables|Default|GetDoorRight)))))

(event EventTick
  (params (DeltaSeconds :type Float%20%28single-precision%29))
  (bind _doortogglecooldown (Variables|Default|GetDoorToggleCooldown))
  (if (> _doortogglecooldown 0)
    (Math|Integer|DecrementInt _doortogglecooldown)))

(event EventInteractEvent
  (params (Requesting%20Player :type Dedicated%20Player%20Controller%20BP%20Object%20Reference))
  (Default|ToggleShopDoors Requesting%20Player self))

(fn ConstructionScript)