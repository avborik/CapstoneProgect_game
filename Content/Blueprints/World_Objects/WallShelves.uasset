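; Wall shelf world object that fills itself with ShelfSlot actors at thirty predefined slot locations.
; On BeginPlay, Init calls PopulateSlotsArray to gather the SlotLocation components into the Slots array.
; It then spawns a ShelfSlot owned by the shelf at each location's world transform, ignoring collisions, and stores the spawned actors in SlotItems.
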(event Custom|Init
  (CallFunction|PopulateSlotsArray)
  (for _array_element (Variables|Default|GetSlots)
    (bind _returnvalue (Game|SpawnActorfromClass "/Game/Blueprints/World_Objects/ShelfSlot.ShelfSlot_C" (Transformation|GetWorldTransform _array_element) "AlwaysSpawn" self 0))
    (Utilities|Array|AddUnique (Variables|Default|GetSlotItems) _returnvalue)))

(event EventBeginPlay
  (CallFunction|Init))

(fn ConstructionScript)

(fn PopulateSlotsArray
  (bind _slots (Variables|Default|GetSlots))
  (Utilities|Array|AddUnique _slots (Variables|Default|GetSlotLocation0))
  (Utilities|Array|AddUnique _slots (Variables|Default|GetSlotLocation1))
  (Utilities|Array|AddUnique _slots (Variables|Default|GetSlotLocation2))
  (Utilities|Array|AddUnique _slots (Variables|Default|GetSlotLocation3))
  (Utilities|Array|AddUnique _slots (Variables|Default|GetSlotLocation4))
  (Utilities|Array|AddUnique _slots (Variables|Default|GetSlotLocation5))
  (Utilities|Array|AddUnique _slots (Variables|Default|GetSlotLocation6))
  (Utilities|Array|AddUnique _slots (Variables|Default|GetSlotLocation7))
  (Utilities|Array|AddUnique _slots (Variables|Default|GetSlotLocation8))
  (Utilities|Array|AddUnique _slots (Variables|Default|GetSlotLocation9))
  (Utilities|Array|AddUnique _slots (Variables|Default|GetSlotLocation10))
  (Utilities|Array|AddUnique _slots (Variables|Default|GetSlotLocation11))
  (Utilities|Array|AddUnique _slots (Variables|Default|GetSlotLocation12))
  (Utilities|Array|AddUnique _slots (Variables|Default|GetSlotLocation13))
  (Utilities|Array|AddUnique _slots (Variables|Default|GetSlotLocation14))
  (Utilities|Array|AddUnique _slots (Variables|Default|GetSlotLocation15))
  (Utilities|Array|AddUnique _slots (Variables|Default|GetSlotLocation16))
  (Utilities|Array|AddUnique _slots (Variables|Default|GetSlotLocation17))
  (Utilities|Array|AddUnique _slots (Variables|Default|GetSlotLocation18))
  (Utilities|Array|AddUnique _slots (Variables|Default|GetSlotLocation19))
  (Utilities|Array|AddUnique _slots (Variables|Default|GetSlotLocation20))
  (Utilities|Array|AddUnique _slots (Variables|Default|GetSlotLocation21))
  (Utilities|Array|AddUnique _slots (Variables|Default|GetSlotLocation22))
  (Utilities|Array|AddUnique _slots (Variables|Default|GetSlotLocation23))
  (Utilities|Array|AddUnique _slots (Variables|Default|GetSlotLocation24))
  (Utilities|Array|AddUnique _slots (Variables|Default|GetSlotLocation25))
  (Utilities|Array|AddUnique _slots (Variables|Default|GetSlotLocation26))
  (Utilities|Array|AddUnique _slots (Variables|Default|GetSlotLocation27))
  (Utilities|Array|AddUnique _slots (Variables|Default|GetSlotLocation28))
  (Utilities|Array|AddUnique _slots (Variables|Default|GetSlotLocation29)))