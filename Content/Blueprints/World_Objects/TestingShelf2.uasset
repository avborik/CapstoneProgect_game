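; TestingShelf2 is a shelf world object that populates four fixed positions with ShelfSlot actors when play begins.
; The construction script gathers the four SlotLocation components into a Slots array, which BeginPlay does not read.
; BeginPlay spawns a slot at each location's world transform, ignoring collisions, and stores each in its own SlotItem variable.
; Only the fourth spawned slot has the shelf set as Owner.
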(event EventBeginPlay
  (bind _returnvalue (Game|SpawnActorfromClass "/Game/Blueprints/World_Objects/ShelfSlot.ShelfSlot_C" (Transformation|GetWorldTransform (Variables|Default|GetSlotLocation0)) "AlwaysSpawn" 0 0))
  (Variables|Default|SetSlotItem0 _returnvalue)
  (bind _returnvalue_2 (Game|SpawnActorfromClass "/Game/Blueprints/World_Objects/ShelfSlot.ShelfSlot_C" (Transformation|GetWorldTransform (Variables|Default|GetSlotLocation1)) "AlwaysSpawn" 0 0))
  (Variables|Default|SetSlotItem1 _returnvalue_2)
  (bind _returnvalue_3 (Game|SpawnActorfromClass "/Game/Blueprints/World_Objects/ShelfSlot.ShelfSlot_C" (Transformation|GetWorldTransform (Variables|Default|GetSlotLocation2)) "AlwaysSpawn" 0 0))
  (Variables|Default|SetSlotItem2 _returnvalue_3)
  (bind _returnvalue_4 (Game|SpawnActorfromClass "/Game/Blueprints/World_Objects/ShelfSlot.ShelfSlot_C" (Transformation|GetWorldTransform (Variables|Default|GetSlotLocation3)) "AlwaysSpawn" self 0))
  (Variables|Default|SetSlotItem3 _returnvalue_4))

(fn ConstructionScript
  (bind _slots (Variables|Default|GetSlots))
  (Utilities|Array|AddUnique _slots (Variables|Default|GetSlotLocation0))
  (Utilities|Array|AddUnique _slots (Variables|Default|GetSlotLocation1))
  (Utilities|Array|AddUnique _slots (Variables|Default|GetSlotLocation2))
  (Utilities|Array|AddUnique _slots (Variables|Default|GetSlotLocation3)))