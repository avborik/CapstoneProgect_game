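; ShelfSlot is a world object that displays the static mesh of an assigned item as a slot on a shelf.
; SetItem checks for a baseObjectActor class, temporarily spawns it, copies its mesh and relative transform onto ItemMesh, then destroys the spawned actor.
; GetParentGUID is unfinished: it only casts the owner to HalfIslandShelves and retrieves no GUID.
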(event Custom|SetItem
  (params (Item :type Base%20Object%20CPP%20Class%20Reference))
  (bind _itemmesh (Variables|Default|GetItemMesh))
  (bind _asbase_object_actor (Utilities|Casting|CastTobaseObjectActorClass Item))
  (bind _output_get (Variables|Default|SetItemClass _asbase_object_actor))
  (bind _returnvalue (Game|SpawnActorfromClass _output_get (Math|Transform|MakeTransform "0, 0, 0") "AlwaysSpawn" 0 0))
  (Components|StaticMesh|SetStaticMesh _itemmesh (Variables|/Script/Engine.StaticMeshComponent|GetStaticMesh (Variables|/Game/Blueprints/Stock_Objects/BaseObject/baseObjectActor.baseObjectActor_C|GetStaticMesh _returnvalue)))
  (Transformation|SetRelativeTransform _itemmesh (Transformation|GetRelativeTransform (Variables|/Game/Blueprints/Stock_Objects/BaseObject/baseObjectActor.baseObjectActor_C|GetStaticMesh _returnvalue)) false true)
  (Actor|DestroyActor _returnvalue))

(event Custom|GetParentGUID
  (Utilities|Casting|CastToHalfIslandShelves (Components|GetOwner)))

(event EventBeginPlay)

(event Collision|EventActorBeginOverlap
  (params (OtherActor :type Actor%20Object%20Reference)))

(event EventTick
  (params (DeltaSeconds :type Float%20%28single-precision%29)))

(fn ConstructionScript)