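; HalfIslandShelves is a world shelf object that creates three slots when play begins.
; BeginPlay calls Init, which spawns a ShelfSlot actor at each of three SlotLocation components, owned by the shelf, and stores them in SlotItem0 to SlotItem2.
; Each slot is set to replicate, though the spawns have no authority check.
; The construction script is empty, and unconnected nodes that would fill a Slots array never run.
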(event Custom|Init
  (bind _returnvalue (Game|SpawnActorfromClass "/Game/Blueprints/World_Objects/ShelfSlot.ShelfSlot_C" (Transformation|GetWorldTransform (Variables|Default|GetSlotLocation1)) "AlwaysSpawn" self 0))
  (Networking|SetReplicates _returnvalue true)
  (Variables|SlotItems|SetSlotItem0 _returnvalue)
  (bind _returnvalue_2 (Game|SpawnActorfromClass "/Game/Blueprints/World_Objects/ShelfSlot.ShelfSlot_C" (Transformation|GetWorldTransform (Variables|Default|GetSlotLocation2)) "AlwaysSpawn" self 0))
  (Networking|SetReplicates _returnvalue_2 true)
  (Variables|SlotItems|SetSlotItem1 _returnvalue_2)
  (bind _returnvalue_3 (Game|SpawnActorfromClass "/Game/Blueprints/World_Objects/ShelfSlot.ShelfSlot_C" (Transformation|GetWorldTransform (Variables|Default|GetSlotLocation3)) "AlwaysSpawn" self 0))
  (Networking|SetReplicates _returnvalue_3 true)
  (Variables|SlotItems|SetSlotItem2 _returnvalue_3))

(event EventBeginPlay
  (CallFunction|Init))

(fn ConstructionScript)