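; Sliding double door actor that opens when an actor overlaps it and closes once no Pawns remain inside its collision component.
; BeginPlay caches both door panels' relative start locations if the left one's stored start is still zero.
; Two timelines, one per panel, add animated vector offsets to those starts, playing forward to open and reversing to close.
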(event EventBeginPlay
  (if (Math|Vector|Equal(Vector) (Variables|Default|GetDoorLeftStartLocation) "0, 0, 0" 0.0001)
    (Variables|Default|SetDoorLeftStartLocation (Variables|/Script/Engine.SceneComponent|GetRelativeLocation (Variables|Default|GetDoorLeft)))
    (Variables|Default|SetDoorRightStartLocation (Variables|/Script/Engine.SceneComponent|GetRelativeLocation (Variables|Default|GetDoorRight)))))

(event Collision|EventActorBeginOverlap
  (params (OtherActor :type Actor%20Object%20Reference))
  (Utilities|FlowControl|Sequence
    (:then_0
      (bind _newtrack_0 (Timeline|Timeline_0 Play)
        (:Update
          (Transformation|SetRelativeLocation (Variables|Default|GetDoorLeft) (+ _newtrack_0 (Variables|Default|GetDoorLeftStartLocation)) false false))))
    (:then_1
      (bind _newtrack_0_2 (Timeline|Timeline_1 Play)
        (:Update
          (Transformation|SetRelativeLocation (Variables|Default|GetDoorRight) (+ _newtrack_0_2 (Variables|Default|GetDoorRightStartLocation)) false false))))))

(event Collision|EventActorEndOverlap
  (params (OtherActor :type Actor%20Object%20Reference))
  (if (== (Utilities|Array|Length (Collision|GetOverlappingActors (Variables|Default|GetCollisionComponent) "/Script/Engine.Pawn" :!class /Script/Engine.PrimitiveComponent)) 0)
    (Utilities|FlowControl|Sequence
      (:then_0
        (bind _newtrack_0 (Timeline|Timeline_0 Reverse)
          (:Update
            (Transformation|SetRelativeLocation (Variables|Default|GetDoorLeft) (+ _newtrack_0 (Variables|Default|GetDoorLeftStartLocation)) false false))))
      (:then_1
        (bind _newtrack_0_2 (Timeline|Timeline_1 Reverse)
          (:Update
            (Transformation|SetRelativeLocation (Variables|Default|GetDoorRight) (+ _newtrack_0_2 (Variables|Default|GetDoorRightStartLocation)) false false)))))))

(fn ConstructionScript)