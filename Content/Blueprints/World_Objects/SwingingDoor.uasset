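; SwingingDoor is a world-object door that swings open when an actor overlaps it and closes when the overlap ends.
; A timeline plays or reverses on overlap, adding its Z rotation track to the stored start yaw to set the Arrow component's world rotation.
; Init runs on BeginPlay, caching the Arrow's start transform and an offset pivot location, which is not used afterwards.
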(event EventBeginPlay
  (CallFunction|Init))

(event Collision|EventActorBeginOverlap
  (params (OtherActor :type Actor%20Object%20Reference))
  (bind _zrotationtrack (Timeline|Timeline_0 Play)
    (:Update
      (Transformation|SetWorldRotation (Variables|Default|GetArrow) (Math|Rotator|MakeRotator 0.0 0.0 (+ _zrotationtrack (.Yaw (Math|Rotator|BreakRotator (Variables|Default|GetdoorStartRotation))))) false false))))

(event Collision|EventActorEndOverlap
  (params (OtherActor :type Actor%20Object%20Reference))
  (bind _zrotationtrack (Timeline|Timeline_0 Reverse)
    (:Update
      (Transformation|SetWorldRotation (Variables|Default|GetArrow) (Math|Rotator|MakeRotator 0.0 0.0 (+ _zrotationtrack (.Yaw (Math|Rotator|BreakRotator (Variables|Default|GetdoorStartRotation))))) false false))))

(event EventTick
  (params (DeltaSeconds :type Float%20%28single-precision%29)))

(fn ConstructionScript)

(fn Init
  (bind _arrow (Variables|Default|GetArrow))
  (bind _returnvalue (Transformation|GetWorldLocation _arrow))
  (bind (_x _y _z) (Math|Vector|BreakVector _returnvalue))
  (if (Math|Vector|Equal(Vector) (Variables|Default|GetdoorStartLocation) "0, 0, 0" 0.0001)
    (Variables|Default|SetdoorStartLocation _returnvalue)
    (Variables|Default|SetdoorSwingPivotLocation (Math|Vector|MakeVector _x (+ _y 5e+01) _z))
    (Variables|Default|SetdoorStartRotation (Transformation|GetWorldRotation (Variables|Default|GetArrow)))))