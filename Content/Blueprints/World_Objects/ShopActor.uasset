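; Player-owned shop actor that builds its interior and displays its security and advertising upgrade levels.
; On BeginPlay, Init spawns replicated door trigger, shelves and cash register at marker components, passing the owner's GUID to the door.
; SetSecurity toggles scanner, cameras or shelf covers (half-island shelf excluded); SetBanner toggles sign, lit posters or lit billboard.
; Tiers are exclusive rather than cumulative, changing only visibility, with no authority check around spawning.
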(event Custom|Init
  (bind _returnvalue (Game|SpawnActorfromClass "/Game/Blueprints/World_Objects/doorTrigger_Blueprint.doorTrigger_Blueprint_C" (Transformation|GetWorldTransform (Variables|StartingLocations|GetDoorLocation)) "AlwaysSpawn" self (Variables|Default|GetOwningPlayerGUID) "Press E to Open Shop" 0))
  (Networking|SetReplicates _returnvalue true)
  (Variables|Default|SetDoor _returnvalue)
  (bind _returnvalue_2 (Game|SpawnActorfromClass "/Game/Blueprints/World_Objects/WallShelves.WallShelves_C" (Transformation|GetWorldTransform (Variables|StartingLocations|GetWallShelfLocation1)) "AlwaysSpawn" self 0))
  (Networking|SetReplicates _returnvalue_2 true)
  (Variables|Shelves|SetWallShelf1 _returnvalue_2)
  (bind _returnvalue_3 (Game|SpawnActorfromClass "/Game/Blueprints/World_Objects/IslandShelves.IslandShelves_C" (Transformation|GetWorldTransform (Variables|StartingLocations|GetIslandShelfLocation1)) "AlwaysSpawn" self 0))
  (Networking|SetReplicates _returnvalue_3 true)
  (Variables|Shelves|SetislandShelf1 _returnvalue_3)
  (bind _returnvalue_4 (Game|SpawnActorfromClass "/Game/Blueprints/World_Objects/IslandShelves.IslandShelves_C" (Transformation|GetWorldTransform (Variables|StartingLocations|GetIslandShelfLocation2)) "AlwaysSpawn" self 0))
  (Networking|SetReplicates _returnvalue_4 true)
  (Variables|Shelves|SetislandShelf2 _returnvalue_4)
  (bind _returnvalue_5 (Game|SpawnActorfromClass "/Game/Blueprints/World_Objects/IslandShelves.IslandShelves_C" (Transformation|GetWorldTransform (Variables|StartingLocations|GetIslandShelfLocation3)) "AlwaysSpawn" self 0))
  (Networking|SetReplicates _returnvalue_5 true)
  (Variables|Shelves|SetislandShelf3 _returnvalue_5)
  (bind _returnvalue_6 (Game|SpawnActorfromClass "/Game/Blueprints/World_Objects/HalfIslandShelves.HalfIslandShelves_C" (Transformation|GetWorldTransform (Variables|Default|GetHalfIslandShelfLocation1)) "AlwaysSpawn" self 0))
  (Networking|SetReplicates _returnvalue_6 true)
  (Variables|Shelves|SetHalfIslandShelf1 _returnvalue_6)
  (bind _returnvalue_7 (Game|SpawnActorfromClass "/Game/Blueprints/World_Objects/CashRegister.CashRegister_C" (Transformation|GetWorldTransform (Variables|StartingLocations|GetCashRegisterLocation)) "AlwaysSpawn" self "Press E to Interact" 0))
  (Networking|SetReplicates _returnvalue_7 true)
  (Variables|Default|SetCashRegister _returnvalue_7))

(event Custom|SetBanner
  (params (BannerLevel :type Integer))
  ;[1 1 1] Banner/Advertising
  (CallFunction|BannerLevel1 (== BannerLevel 1))
  (CallFunction|BannerLevel2 (== BannerLevel 2))
  (CallFunction|BannerLevel3 (== BannerLevel 3)))

(event Custom|BannerLevel1
  (params (Enable :type Boolean))
  ;[1 1 1] Banner/Advertising
  (Rendering|SetVisibility (Variables|Banners|GetBannerSign) Enable false))

(event Custom|BannerLevel2
  (params (Enable :type Boolean))
  ;[1 1 1] Banner/Advertising
  (Utilities|FlowControl|Sequence
    (:then_0
      (Rendering|SetVisibility (Variables|Banners|GetBannerPoster1) Enable false)
      (Rendering|SetVisibility (Variables|Banners|GetBannerPoster2) Enable false)
      (Rendering|SetVisibility (Variables|Banners|GetBannerPoster3) Enable false)
      (Rendering|SetVisibility (Variables|Banners|GetBannerPoster4) Enable false))
    (:then_1
      (Rendering|SetVisibility (Variables|BannerLights|GetPosterLight1) Enable false)
      (Rendering|SetVisibility (Variables|BannerLights|GetPosterLight2) Enable false)
      (Rendering|SetVisibility (Variables|BannerLights|GetPosterLight3) Enable false)
      (Rendering|SetVisibility (Variables|BannerLights|GetPosterLight4) Enable false))))

(event Custom|BannerLevel3
  (params (Enable :type Boolean))
  ;[1 1 1] Banner/Advertising
  (Rendering|SetVisibility (Variables|Banners|GetBannerBillboard) Enable false)
  (Rendering|SetVisibility (Variables|BannerLights|GetbillboardLight1) Enable false)
  (Rendering|SetVisibility (Variables|BannerLights|GetbillboardLight2) Enable false)
  (Rendering|SetVisibility (Variables|BannerLights|GetbillboardLight3) Enable false)
  (Rendering|SetVisibility (Variables|BannerLights|GetbillboardLight4) Enable false)
  (Rendering|SetVisibility (Variables|BannerLights|GetbillboardLight5) Enable false))

(event Custom|SetSecurity
  (params (SecurityLevel :type Integer))
  ;[1 1 1] Security
  (CallFunction|SecurityLevel1 (== SecurityLevel 1))
  (CallFunction|SecurityLevel2 (== SecurityLevel 2))
  (CallFunction|SecurityLevel3 (== SecurityLevel 3)))

(event Custom|SecurityLevel3
  (params (Enable :type Boolean))
  ;[1 1 1] Security
  (Rendering|SetVisibility (Variables|/Game/Blueprints/World_Objects/WallShelves.WallShelves_C|GetSecurityCover (Variables|Shelves|GetWallShelf1)) Enable false)
  (Rendering|SetVisibility (Variables|/Game/Blueprints/World_Objects/IslandShelves.IslandShelves_C|GetSecurityCover (Variables|Shelves|GetislandShelf1)) Enable false)
  (Rendering|SetVisibility (Variables|/Game/Blueprints/World_Objects/IslandShelves.IslandShelves_C|GetSecurityCover (Variables|Shelves|GetislandShelf2)) Enable false)
  (Rendering|SetVisibility (Variables|/Game/Blueprints/World_Objects/IslandShelves.IslandShelves_C|GetSecurityCover (Variables|Shelves|GetislandShelf3)) Enable false))

(event Custom|SecurityLevel2
  (params (Enable :type Boolean))
  ;[1 1 1] Security
  (Rendering|SetVisibility (Variables|Security|GetSecurityCamera1) Enable false)
  (Rendering|SetVisibility (Variables|Security|GetSecurityCamera2) Enable false)
  (Rendering|SetVisibility (Variables|Security|GetSecurityCamera3) Enable false))

(event Custom|SecurityLevel1
  (params (Enable :type Boolean))
  ;[1 1 1] Security
  (Rendering|SetVisibility (Variables|Security|GetSecurityScanner1) Enable false))

(event EventBeginPlay
  (CallFunction|Init)
  (CallFunction|SetSecurity (Variables|Default|GetSecurityLevel))
  (CallFunction|SetBanner (Variables|Default|GetBannerLevel)))

(fn ConstructionScript)