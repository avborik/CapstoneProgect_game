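; Player controller for a dedicated-server game, managing a player's persistent data, inventory and item placement on shelves.
; BeginPlay passes the session GUID to the server, spawns the inventory actor and loads currency, security level and items over REST.
; Authority-checked functions change inventory and push slot updates to the HUD hotbar; PlaceItem moves items to or from shelf slots.
; Saving only builds and prints JSON, never sending it; slot insertion is stubbed.
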(event Custom|GetPlayerDetails
  ;[1 1 1] Get data from db for joined player
  (Variables|Default|SetVaRequest_Load (Class|VaRestRequestJSON|ConstructRequestExt "GET" "x_www_form_urlencoded_url"))
  (EventDispatchers|BindEventtoOnRequestFail (Variables|Default|GetVaRequest_Load) (delegate Custom|OnRequestFail))
  (EventDispatchers|BindEventtoOnRequestComplete (Variables|Default|GetVaRequest_Load) (delegate Custom|OnRequestComplete))
  (bind _returnvalue (Class|VaRestRequestJSON|GetRequestObject (Variables|Default|GetVaRequest_Load)))
  (Class|VaRestJsonObject|SetStringField _returnvalue "getPlayerData" (Variables|Default|GetGUIDString))
  (Class|VaRestRequestJSON|ProcessURL (Variables|Default|GetVaRequest_Load) "schollitt.com/rest/rest.php"))

(event Custom|OnRequestComplete
  (params (Request :type Va%20Rest%20Request%20JSON%20Object%20Reference))
  ;[1 1 1] Get data from db for joined player
  (bind _returnvalue (Class|VaRestRequestJSON|GetResponseObject Request))
  (Utilities|Casting|CastToDedicatedPlayerStateBP (Variables|Default|GetPlayerState))
  (Variables|ClientPrivate|SetCurrency (Math|Conversions|ToFloat(Integer) (Class|VaRestJsonObject|GetStringField _returnvalue "currency")))
  (Variables|ClientPrivate|SetSecurityLevel (Math|Conversions|ToInteger(Byte) (Class|VaRestJsonObject|GetStringField _returnvalue "security")))
  (for _array_element (Class|VaRestJsonObject|GetArrayField _returnvalue "inventory")
    (bind _returnvalue_2 (Class|VaRestJsonValue|AsObject _array_element))
    (bind _asdedicated_game_instance_bp (Utilities|Casting|CastToDedicatedGameInstanceBP (Game|GetGameInstance)))
    (bind _returnvalue_3 (Class|DedicatedGameInstance|GetItemClassfromID _asdedicated_game_instance_bp "/Game/Blueprints/Stock_Objects/BaseObject/shopItemsLibrary.shopItemsLibrary" (Math|Conversions|ToInteger(Byte) (Class|VaRestJsonObject|GetStringField _returnvalue_2 "id"))))
    (bind _asbase_object_actor (Utilities|Casting|CastTobaseObjectActorClass _returnvalue_3))
    (CallFunction|ServerSetItemSlot _asbase_object_actor (Math|Conversions|ToInteger(Byte) (Class|VaRestJsonObject|GetStringField _returnvalue_2 "slot")) (Math|Conversions|ToInteger(Byte) (Class|VaRestJsonObject|GetStringField _returnvalue_2 "quantity")))))

(event Custom|SaveDataFailed
  (params (Request :type Va%20Rest%20Request%20JSON%20Object%20Reference))
  ;[1 1 1] Save Data on player leave
)

(event Custom|SaveDataSucceeded
  (params (Request :type Va%20Rest%20Request%20JSON%20Object%20Reference))
  ;[1 1 1] Save Data on player leave
)

(event Custom|OnRequestFail
  (params (Request :type Va%20Rest%20Request%20JSON%20Object%20Reference))
  ;[1 1 1] Get data from db for joined player
  (Development|PrintString "Request for player data failed")
  (|Logout self))

(event Custom|SetGUIDServer
  (params (GUIDString :type String))
  ;[1 1 1] Set the GUID to the replicated variable from the client
  (bind _output_get (Variables|Default|SetGUIDString GUIDString))
  (Development|PrintString (Utilities|String|Append "GUID server: " _output_get) true true "(R=0.889269,G=0.923991,B=1.000000,A=1.000000)" 3e+01))

(event Custom|testing
  (params (NewParam :type Integer)))

(event Custom|InitPlayerInventory
  ;[-0.2476 1 -0.2952] Inventory related
  ;;[1 1 1] Spawn inventory actor as child of controller and save reference to variable
  (Networking|SwitchHasAuthority
    (:Authority
      (Utilities|IsValid (Variables|ClientPrivate|GetplayerInventory)
        (:Is%20Not%20Valid
          (bind _returnvalue (Game|SpawnActorfromClass "/Game/Blueprints/inventory/BaseInventory.BaseInventory_C" (Math|Transform|MakeTransform "0, 0, 0") "AlwaysSpawn" self 1e+02 (Variables|Default|GetInventorySlotCount) 0))
          (bind _output_get (Variables|ClientPrivate|SetplayerInventory _returnvalue))
          (Utilities|IsValid _output_get
            (:Is%20Valid
              (Default|Init _output_get))
            (:Is%20Not%20Valid
              (Development|PrintString "Inventory did not init"))))))))

(event Custom|ClientPlaceItem
  ;[1 1 1] Client side
  (bind _asdedicated_game_hud (Utilities|Casting|CastToDedicatedGameHUD (HUD|GetHUD)))
  (bind _asdedicated_character_bp (Utilities|Casting|CastToDedicatedCharacterBP (Game|GetPlayerCharacter 0)))
  (if (Variables|/Game/Blueprints/Character/DedicatedCharacterBP.DedicatedCharacterBP_C|GetIsLookingAtShelfSlot _asdedicated_character_bp)
    (CallFunction|ServerPlaceItem (Variables|/Game/Blueprints/HUD/HotbarWidget.HotbarWidget_C|GetHighlightedIndex (Variables|/Game/Blueprints/HUD/DedicatedGameHUD.DedicatedGameHUD_C|GetHotbarWidget _asdedicated_game_hud)) (Variables|/Game/Blueprints/Character/DedicatedCharacterBP.DedicatedCharacterBP_C|GetlastHit _asdedicated_character_bp))))

(event Custom|SaveDataToServer
  ;[1 1 1] Save Data on player leave
  (bind _output_get (Variables|Default|SetVaRequest_Save (Class|VaRestRequestJSON|ConstructRequestExt "GET" "x_www_form_urlencoded_body")))
  (EventDispatchers|BindEventtoOnRequestFail _output_get (delegate Custom|SaveDataFailed))
  (EventDispatchers|BindEventtoOnRequestFail _output_get (delegate Custom|SaveDataSucceeded))
  (bind _returnvalue (Class|VaRestRequestJSON|GetRequestObject _output_get))
  (Class|VaRestJsonObject|SetStringField _returnvalue "guid" (Variables|Default|GetGUIDString))
  (Class|VaRestJsonObject|SetStringField _returnvalue "display")
  (Class|VaRestJsonObject|SetStringField _returnvalue "currency" (Utilities|String|ToString(Float) (Variables|ClientPrivate|GetCurrency)))
  (Class|VaRestJsonObject|SetStringField _returnvalue "security" (Utilities|String|ToString(Integer) (Variables|ClientPrivate|GetSecurityLevel)))
  (Class|VaRestJsonObject|SetStringField _returnvalue "rent" (Utilities|String|ToString(Float) (Variables|ClientPrivate|GetRentCredit)))
  (for (_array_element _array_index) (Variables|/Game/Blueprints/inventory/BaseInventory.BaseInventory_C|GetInvSlots (Variables|ClientPrivate|GetplayerInventory))
    (Class|VaRestJsonObject|SetStringField _returnvalue (Utilities|String|BuildString(Integer) "" "item_" _array_index) (Utilities|String|Append (Utilities|String|ToString(Integer) (.ObjectID (Utilities|GetClassDefaults (.ItemType (Utilities|Struct|BreakInventoryStruct _array_element))))) "," (Utilities|String|ToString(Integer) (.StackCount (Utilities|Struct|BreakInventoryStruct _array_element))) "," (Utilities|String|ToString(Integer) _array_index))))
  (Development|PrintString (Class|VaRestJsonObject|EncodeJson _returnvalue)))

(event Custom|ServerPlaceItem
  (params (InventoryIndex :type Integer) (ShelfSlot :type Shelf%20Slot%20Object%20Reference))
  (bind _playerinventory (Variables|ClientPrivate|GetplayerInventory))
  (bind _itemclass (Variables|/Game/Blueprints/World_Objects/ShelfSlot.ShelfSlot_C|GetItemClass ShelfSlot))
  (bind _invslots (Variables|/Game/Blueprints/inventory/BaseInventory.BaseInventory_C|GetInvSlots _playerinventory))
  (bind _output (Utilities|Array|Get(acopy) _invslots InventoryIndex))
  (bind (_itemtype _stackcount) (Utilities|Struct|BreakInventoryStruct _output))
  (if (== _itemclass "/Game/Blueprints/Stock_Objects/BaseObject/emptyObject.emptyObject_C")
    (if (!= _itemtype "/Game/Blueprints/Stock_Objects/BaseObject/emptyObject.emptyObject_C")
      (if (> _stackcount 0)
        (Default|SetItem ShelfSlot _itemtype)
        (CallFunction|ServerRemoveItemfromSlot InventoryIndex)
        (else
          (Development|PrintString "inv slot stack = 0, this SHOULD NOT happen"))))
    (else
      (bind _successful (CallFunction|ServerAddItem _itemclass))
      (if _successful
        (Default|SetItem ShelfSlot "/Game/Blueprints/Stock_Objects/BaseObject/emptyObject.emptyObject_C")
        (else
          (Development|PrintString "Inventory is full, cannot remove item from the shelf"))))))

(event Custom|ClientUpdateInventorySlot
  (params (SlotIndex :type Integer) (inventory :type Inventory%20Struct%20Structure))
  (bind (_itemtype _stackcount) (Utilities|Struct|BreakInventoryStruct inventory))
  ;[1 1 1] Client side
  ;;[1 1 1] Set inventory slot based on inventory class from server
  (bind _asdedicated_game_hud (Utilities|Casting|CastToDedicatedGameHUD (HUD|GetHUD)))
  (Default|SetSlot (Variables|/Game/Blueprints/HUD/DedicatedGameHUD.DedicatedGameHUD_C|GetHotbarWidget _asdedicated_game_hud) SlotIndex (Utilities|Struct|BreakImageContainer (.ImageContainer (Utilities|GetClassDefaults _itemtype))) _stackcount))

(event EventBeginPlay
  (bind (_isvalid _returnvalue) (Class|PlayerSessionSingleton|GetPlayerSessionSingleton))
  ;[1 1 1] initialise
  (if (Pawn|IsLocalPlayerController)
    (if _isvalid
      (bind _returnvalue_2 (Class|PlayerSessionVariables|GetGUID _returnvalue))
      (Development|PrintString _returnvalue_2 true true "(R=0.701023,G=0.000000,B=1.000000,A=1.000000)" 3e+01)
      (CallFunction|SetGUIDServer _returnvalue_2)
      (CallFunction|InitPlayerInventory)
      (CallFunction|GetPlayerDetails)
      (else
        (Development|PrintString "GUID singleton failed" true true "(R=1.000000,G=0.000000,B=0.000000,A=1.000000)" 3e+01)))))

(event EventEndPlay
  (params (EndPlayReason :type EEndPlayReason%20Enum :default "Destroyed"))
  (CallFunction|SaveDatatoServer))

(event Input|ActionEvents|InputActionPlaceItem
  (params (Key :type Key%20Structure))
  ;[1 1 1] Client side
  (:Pressed
    (CallFunction|ClientPlaceItem)))

(event Input|KeyboardEvents|B
  (params (Key :type Key%20Structure))
  ;[1 1 1] Save Data on player leave
  (:Pressed
    (CallFunction|SaveDatatoServer)))

(event Input|KeyboardEvents|Escape
  (params (Key :type Key%20Structure))
  ;[1 1 1] Client side
  ;;[1 1 1] Show the ingame escape menu
  (:Pressed
    (bind _returnvalue (UserInterface|CreateWidget "/Game/Blueprints/HUD/InGameEscapeMenuWidget.InGameEscapeMenuWidget_C" self))
    (UserInterface|Viewport|AddtoViewport _returnvalue 0)
    (Input|SetInputModeUIOnly self _returnvalue "DoNotLock")))

(event Input|KeyboardEvents|Z
  (params (Key :type Key%20Structure))
  (:Pressed
    (CallFunction|Testing 9)))

(fn ConstructionScript)

(fn RemoveItemfromInventory
  (params (Slot%20index :type Integer) (NewParam1 :type Base%20Object%20Actor%20Class%20Reference))
  ;[1 1 1] Server only
  (Networking|SwitchHasAuthority
    (:Authority
      (Default|RemoveItem (Variables|ClientPrivate|GetplayerInventory) Slot%20index)
      (CallFunction|ClientUpdateInventorySlot Slot%20index (Utilities|Array|Get(acopy) (Variables|/Game/Blueprints/inventory/BaseInventory.BaseInventory_C|GetInvSlots (Variables|ClientPrivate|GetplayerInventory)) Slot%20index)))))

(fn InsertItemIntoInventory
  (params (ItemToAdd :type Base%20Object%20Actor%20Class%20Reference) (Index :type Integer) (ForceReplace :type Boolean))
  (Networking|SwitchHasAuthority
    (:Authority
      (return false false))))

(fn DropItemfromInventory)

(fn UpdateItemList)

(fn ServerAddItemtoSlot
  (params (ItemToAdd :type Base%20Object%20Actor%20Class%20Reference) (Slot :type Integer) (ForceReplace :type Boolean))
  (Networking|SwitchHasAuthority
    (:Authority
      (bind (_inserted _notforcedslotoccupied) (CallFunction|InsertItemIntoInventory ItemToAdd Slot ForceReplace))
      (if _notforcedslotoccupied
        (Development|PrintString "Failed to insert, slot occupied")
        (elif _inserted
          (return true)
          (else
            (Development|PrintString "Failed to insert item into inventory"))))
      (return false))))

(fn ServerAddItem
  (params (ItemToAdd :type Base%20Object%20CPP%20Class%20Reference))
  (bind _playerinventory (Variables|ClientPrivate|GetplayerInventory))
  (Networking|SwitchHasAuthority
    (:Authority
      (bind (_wasadded _newitemindex) (Default|AddItemtoInventory _playerinventory ItemToAdd))
      (if _wasadded
        (CallFunction|ClientUpdateInventorySlot _newitemindex (Utilities|Array|Get(acopy) (Variables|/Game/Blueprints/inventory/BaseInventory.BaseInventory_C|GetInvSlots _playerinventory) _newitemindex))
        (return true)
        (else
          (return false))))))

(fn ServerSetItemSlot
  (params (Item :type Base%20Object%20CPP%20Class%20Reference) (Slot%20Number :type Integer) (Quantity :type Integer))
  (bind _playerinventory (Variables|ClientPrivate|GetplayerInventory))
  (Networking|SwitchHasAuthority
    (:Authority
      (bind (_set_item _slot1) (Default|SetItemSlot _playerinventory Item Slot%20Number Quantity false))
      (CallFunction|ClientUpdateInventorySlot _slot1 _set_item)
      (Default|PrintInventory _playerinventory))))

(fn ServerRemoveItemfromSlot
  (params (Slot%20index :type Integer))
  (Networking|SwitchHasAuthority
    (:Authority
      (CallFunction|RemoveItemfromInventory Slot%20index))))